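; Behavior Tree task for Enemy1 that increments the blackboard path index used with the enemy's WallJumpPoints path.
; It compares the next index to the last PathPoints index and increments only when the next index is at or past that last one.
; It finishes successfully after incrementing; a failed cast or unmet condition leaves the task without a FinishExecute call.
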(event `self.ReceiveExecuteAI`
  (params (OwnerController :type "AIController Object Reference") (ControlledPawn :type "Pawn Object Reference"))
  (bind _returnvalue (+ (`BTFunctionLibrary.GetBlackboardValueAsInt` (`self.BB_PathIndex`)) 1))
  (bind _asenemy_1 (cast `/Game/Character/Blueprints/Enemies/Enemy1` ControlledPawn))
  (if (<= (- (`KismetArrayLibrary.Array_Length` (`/Game/Character/Blueprints/Enemies/WallJumpActor.PathPoints` (`/Game/Character/Blueprints/Enemies/Enemy1.WallJumpPoints` _asenemy_1))) 1) _returnvalue)
    (`BTFunctionLibrary.SetBlackboardValueAsInt` (`self.BB_PathIndex`) _returnvalue)
    (`self.FinishExecute` true)))