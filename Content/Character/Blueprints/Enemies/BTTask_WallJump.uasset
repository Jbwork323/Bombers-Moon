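; Behavior Tree task that supplies the next wall jump location for an Enemy1 pawn.
; It reads the path index from the Blackboard, transforms that entry of the pawn's WallJumpPoints actor from local to world space, and writes it to the path vector key.
; It finishes successfully only when the points actor is valid; a failed cast or invalid actor never calls FinishExecute.
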(event `self.ReceiveExecuteAI`
  (params (OwnerController :type "AIController Object Reference") (ControlledPawn :type "Pawn Object Reference"))
  (bind _asenemy_1 (cast `/Game/Character/Blueprints/Enemies/Enemy1` ControlledPawn))
  (bind _walljumppoints (`/Game/Character/Blueprints/Enemies/Enemy1.WallJumpPoints` _asenemy_1)
    (:`then`
      (`BTFunctionLibrary.SetBlackboardValueAsVector` (`self.BB_PathVector`) (`KismetMathLibrary.TransformLocation` (`Actor.GetTransform` _walljumppoints) (`|GetArrayItem` (`/Game/Character/Blueprints/Enemies/WallJumpActor.PathPoints` _walljumppoints) (`BTFunctionLibrary.GetBlackboardValueAsInt` (`self.BB_PathIndex`)))))
      (`self.FinishExecute` true))
    (:`else`)))