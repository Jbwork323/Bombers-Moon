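; Enemy character that initializes its health, tells its IC_Enemy1 AI controller to attack when the player enters its box, and destroys itself on Tick once health runs out.
; Helpers set walk speed and launch a wall jump with gravity disabled, using absolute velocities derived from a timed arc formula.
; An old projectile line trace that sets the PlayerInRange blackboard key for a distant player remains, but its EventGraph caller is disconnected.
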(event `self.ReceiveBeginPlay`
  (set `self.CurrentHealth` (`self.MaxHealth`)))

(event `self.Box.OnComponentBeginOverlap`
  (params (OverlappedComponent :type "PrimitiveComponent Object Reference") (OtherActor :type "Actor Object Reference") (OtherComp :type "PrimitiveComponent Object Reference") (OtherBodyIndex :type Integer) (bFromSweep :type Boolean) (SweepResult :type "HitResult Structure (by ref)"))
  ;[1 1 1] Attacking Detection
  (if (== OtherActor (`GameplayStatics.GetPlayerCharacter` 0))
    (`/Game/Character/Blueprints/Enemies/AIC_Enemy1.Attacking` (cast `/Game/Character/Blueprints/Enemies/AIC_Enemy1` (`self.GetController`) :!pure true))
    (`ActorComponent.Deactivate` (`self.Box`))))

(event `self.ReceiveTick`
  (params (DeltaSeconds :type "Float (single-precision)"))
  (if (<= (`self.CurrentHealth`) 0.0)
    (set `self.AIControllerClass` "/Script/AIModule.AIController")
    (`self.K2_DestroyActor`)
    (`self.K2_DestroyActor`)))

(fn `LineTraceForProjectileLogic`
  (bind _location (.location (`SceneComponent.K2_GetComponentToWorld` (`self.Cube`))))
  (bind _blackboard (`AIController.Blackboard` (`AIBlueprintHelperLibrary.GetAIController` self)))
  (bind _outhit (`KismetSystemLibrary.LineTraceSingleForObjects` _location (+ _location (* (`KismetMathLibrary.GetForwardVector` (.rotation (`SceneComponent.K2_GetComponentToWorld` (`self.Cube`)))) 1500.0)) (`|MakeArray` "ObjectTypeQuery3" :!type "EObjectTypeQuery Enum")))
  (if (and (== (`.HitActor` (`GameplayStatics.BreakHitResult` _outhit)) (`GameplayStatics.GetPlayerCharacter` 0)) (> (`self.GetDistanceTo` (`GameplayStatics.GetPlayerCharacter` 0)) 500.0))
    (`BlackboardComponent.SetValueAsBool` _blackboard (`self.PlayerInRange`) true)
    (else
      (`BlackboardComponent.SetValueAsBool` _blackboard (`self.PlayerInRange`) false))))

(fn `UpdateWalkSpeed`
  (params (NewWalkSpeed :type "Float (double-precision)"))
  (set `CharacterMovementComponent.MaxWalkSpeed` NewWalkSpeed (`self.CharacterMovement`)))

(fn `UserConstructionScript`)

(fn `WallJumpFunction`
  (params (PathPointLocation :type "Vector Structure") (StartingLocation :type "Vector Structure"))
  (returns (Velocity :type "Vector Structure"))
  (locals (Duration :type "Float (double-precision)" :default 2.0))
  (bind _duration (`local.Duration`))
  (`PrimitiveComponent.SetEnableGravity` (`self.CapsuleComponent`) false)
  (`MovementComponent.StopMovementImmediately` (`self.CharacterMovement`))
  (`self.LaunchCharacter` (`KismetMathLibrary.MakeVector` (`KismetMathLibrary.Abs` (/ (- (.x PathPointLocation) (.x StartingLocation)) _duration)) (`KismetMathLibrary.Abs` (/ (- (.y PathPointLocation) (.y StartingLocation)) _duration)) (`KismetMathLibrary.Abs` (/ (- (.z PathPointLocation) (+ (.z StartingLocation) (* (`KismetMathLibrary.Square` (`local.Duration`)) -0.5 982.0))) (`local.Duration`)))) true true)
  (return (0.0 0.0 0.0)))