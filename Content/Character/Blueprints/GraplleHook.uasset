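; Grappling hook actor for ColorSwapCharacter, drawn with a cable attached to the player character.
; Each tick it traces back to the player; hitting a "Grapple"-tagged actor passes the hit to the character, flags it as grappled and destroys the hook.
; A collision Hit also destroys the hook without grappling, and destruction clears the character's GrappleInAir flag.
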(event `self.ReceiveBeginPlay`
  (`CableComponent.SetAttachEndTo` (`self.Cable`) (`GameplayStatics.GetPlayerCharacter` 0) "None" "None"))

(event `self.ReceiveTick`
  (params (DeltaSeconds :type "Float (single-precision)"))
  (bind _returnvalue (`GameplayStatics.GetPlayerCharacter` 0))
  (bind (_outhit _returnvalue_2) (`KismetSystemLibrary.LineTraceSingle` (`self.K2_GetActorLocation`) (`self.K2_GetActorLocation` _returnvalue) "TraceTypeQuery1" false (`|MakeArray` _returnvalue)))
  (if _returnvalue_2
    (bind _ascolor_swap_character (cast `/Game/Character/Blueprints/ColorSwapCharacter` (`GameplayStatics.GetPlayerCharacter` 0)))
    (if (`self.ActorHasTag` (`.HitActor` (`GameplayStatics.BreakHitResult` _outhit)) "Grapple")
      (set `/Game/Character/Blueprints/ColorSwapCharacter.IsGrapped` true _ascolor_swap_character)
      (set `/Game/Character/Blueprints/ColorSwapCharacter.GrappleHit` _outhit _ascolor_swap_character)
      (`self.K2_DestroyActor` :!label _label))))

(event `self.ReceiveHit`
  (params (MyComp :type "PrimitiveComponent Object Reference") (Other :type "Actor Object Reference") (OtherComp :type "PrimitiveComponent Object Reference") (bSelfMoved :type Boolean) (HitLocation :type "Vector Structure") (HitNormal :type "Vector Structure") (NormalImpulse :type "Vector Structure") (Hit :type "HitResult Structure (by ref)"))
  (goto _label))

(event `self.ReceiveDestroyed`
  (bind _ascolor_swap_character (cast `/Game/Character/Blueprints/ColorSwapCharacter` (`GameplayStatics.GetPlayerCharacter` 0)))
  (set `/Game/Character/Blueprints/ColorSwapCharacter.GrappleInAir` false _ascolor_swap_character))

(fn `UserConstructionScript`)