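; ColorBase_BP is a colored platform for the color-change mechanic, present only while its color is active.
; Its construction script applies the chosen mesh to the Cube and picks a material from the Color enum.
; ChangeToColor shows the actor with collision on a color match, otherwise hides it and disables collision.
; A Fire input triggers this update only when its OnlyCertainColor flag is set; other inputs always do.
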(fn `Change To Color`
  (params (`Active Color` :type "/Game/Character/Blueprints/ColorEnum Enum" :default "NewEnumerator5") (Input :type "/Game/ColorChangeMechanics/Platforms/BasicPlatforms/ColorBase_BP Object Reference"))
  (bind _asfire (cast `/Game/OtherThings/Fire` Input)
    (:`then`
      (if (`/Game/OtherThings/Fire.OnlyCertainColor` _asfire)
        (if (== `Active Color` (`self.Color`)) :!label _label
          (`self.SetActorHiddenInGame` false)
          (`PrimitiveComponent.SetCollisionEnabled` (`self.Cube`) "QueryAndPhysics")
          (else
            (`self.SetActorHiddenInGame` true)
            (`PrimitiveComponent.SetCollisionEnabled` (`self.Cube`) "NoCollision")))))
    (:`CastFailed`
      (goto _label))))

(fn `UserConstructionScript`
  (bind _cube (`self.Cube`))
  (`PrimitiveComponent.SetMaterial` _cube 0 (select `/Game/Character/Blueprints/ColorEnum` (`self.Color`) :`NewEnumerator5` "/Game/StarterContent/Materials/M_Basic_Floor.M_Basic_Floor" :`NewEnumerator0` "/Game/ColorChangeMechanics/Platforms/Matterials/Red.Red" :`NewEnumerator1` "/Game/ColorChangeMechanics/Platforms/Matterials/Blue.Blue" :`NewEnumerator2` "/Game/ColorChangeMechanics/Platforms/Matterials/Yellow.Yellow" :!type "MaterialInterface Object Reference"))
  (`StaticMeshComponent.SetStaticMesh` _cube (`self.Mesh`)))