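; Shop actor that opens a purchase menu when the player presses interact while inside its overlap area.
; Tick polls the character's Interact value through a Gate opened by overlap, with a DoOnce limiting creation to one widget per visit.
; The Shop widget receives item names, images, prices and stock, animates in and enables the cursor.
; Leaving the area animates it out, removes it and restores game-only input.
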(event `self.ReceiveTick`
  (params (DeltaSeconds :type "Float (single-precision)"))
  (bind _returnvalue (`GameplayStatics.GetPlayerController` 0))
  ;[1 1 1] Controls opening and closing the shop
  (bind _ascolor_swap_character (cast `/Game/Character/Blueprints/ColorSwapCharacter` (`GameplayStatics.GetPlayerCharacter` 0)))
  (bind _interating (`/Game/Character/Blueprints/ColorSwapCharacter.Interact` _ascolor_swap_character))
  (if _interating
    (`/Engine/EditorBlueprintResources/StandardMacros.Gate` true :!label _label
      (:`Exit`
        (`/Engine/EditorBlueprintResources/StandardMacros.DoOnce` false :!label _label_2
          (:`Completed`
            (`|ExecutionSequence`
              (:`then_0`
                (cast `/Game/Character/Blueprints/ColorSwapCharacter` (stale `self.ReceiveActorBeginOverlap` OtherActor))
                (bind _returnvalue_2 (`|CreateWidget` "/Game/ColorChangeMechanics/UI/Shop.Shop_C" _returnvalue))
                (bind _output_get (set `self.Shop` _returnvalue_2))
                (`UserWidget.AddToViewport` _output_get 0)
                (`UserWidget.PlayAnimation` _output_get (`/Game/ColorChangeMechanics/UI/Shop.ShopClose` _output_get) 0.0 1 "Reverse" 1.0 false)
                (`/Game/ColorChangeMechanics/UI/Shop.ShopInitiate` _output_get (`self.Item Names`) (`self.ImageArray`) (`self.Prices`) (`self.Stock`))
                (`WidgetBlueprintLibrary.SetInputMode_GameAndUIEx` _returnvalue _output_get)
                (set `PlayerController.bShowMouseCursor` true _returnvalue))
              (:`then_1`
                (goto _label_3 :!via `Reset`)))))))))

(event `self.ReceiveActorBeginOverlap`
  (params (OtherActor :type "Actor Object Reference"))
  ;[1 1 1] Controls opening and closing the shop
  (goto _label :!via `Open`))

(event `self.ReceiveActorEndOverlap`
  (params (OtherActor :type "Actor Object Reference"))
  (bind _returnvalue (`GameplayStatics.GetPlayerController` 0))
  ;[1 1 1] Controls opening and closing the shop
  (`|ExecutionSequence`
    (:`then_0`
      (goto _label :!via `Close`))
    (:`then_1`
      (goto _label_2 :!via `Reset`))
    (:`then_2`
      (cast `/Game/Character/Blueprints/ColorSwapCharacter` OtherActor)
      (`/Engine/EditorBlueprintResources/StandardMacros.DoOnce` true :!label _label_3
        (:`Completed`
          (`|ExecutionSequence`
            (:`then_0`
              (`UserWidget.PlayAnimation` (stale `self.ReceiveTick` _output_get) (`/Game/ColorChangeMechanics/UI/Shop.ShopClose` (stale `self.ReceiveTick` _output_get)) 0.0 1 "Forward" 1.0 false)
              (`KismetSystemLibrary.Delay` 1.0)
              (`Widget.RemoveFromParent` (stale `self.ReceiveTick` _output_get)))
            (:`then_1`
              (`WidgetBlueprintLibrary.SetInputMode_GameOnly` _returnvalue)
              (set `PlayerController.bShowMouseCursor` false _returnvalue))))))))

(fn `UserConstructionScript`)