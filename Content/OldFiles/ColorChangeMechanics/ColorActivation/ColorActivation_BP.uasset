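; ColorActivation_BP is an actor whose particle effect matches its assigned color.
; A map looks up the particle template for the Color variable and sets it on the Particles component.
; The same lookup runs in the construction script and in a Build event.
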(event `Build`
  ;[1 1 1] Changes particles to what color they're set
  (`ParticleSystemComponent.SetTemplate` (`self.Particles`) (`BlueprintMapLibrary.Map_Find` (`self.ColorMap`) (`self.Color`))))

(fn `UserConstructionScript`
  ;[1 1 1] Changes Particles to what color they're set to when constructed
  (`ParticleSystemComponent.SetTemplate` (`self.Particles`) (`BlueprintMapLibrary.Map_Find` (`self.ColorMap`) (`self.Color`))))