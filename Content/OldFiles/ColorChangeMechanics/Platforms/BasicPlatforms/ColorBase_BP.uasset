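; Base color-coded platform that appears or disappears as the active color in the game changes.
; Construction applies the material for its Color and the chosen mesh, showing either the mesh or a Selector per IsVisible; BeginPlay always reveals the mesh.
; ChangeToColor toggles actor visibility and collision together by color match, inverted when AppearsOnActive is off.
; Fire inputs trigger this only when flagged OnlyCertainColor.
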(event `self.ReceiveBeginPlay`
  ;[1 1 1] Makes the mesh visible on BeginPlay
  (`SceneComponent.SetVisibility` (`self.StaticMesh`) true true))

(fn `Change To Color`
  (params (`Active Color` :type "/Game/OldFiles/Character/Blueprints/ColorEnum Enum" :default "NewEnumerator5") (Input :type "/Game/OldFiles/ColorChangeMechanics/Platforms/BasicPlatforms/ColorBase_BP Object Reference"))
  (bind _returnvalue (== `Active Color` (`self.Color`)))
  ;[1 1 1] Checks fires to see we want them to be affected by color changes
  (bind _asfire (cast `/Game/OldFiles/LevelBuildingBlueprints/Fire` Input)
    (:`then`
      (if (`/Game/OldFiles/LevelBuildingBlueprints/Fire.OnlyCertainColor` _asfire)
        ;[1 1 1] Sets the correct visibility and collision based on the color in game and whether it appears on active
        (if (`self.AppearsOnActive`) :!label _label
          (if _returnvalue
            (`self.SetActorHiddenInGame` false :!label _label_2)
            (`self.SetActorEnableCollision` true)
            (else
              (`self.SetActorHiddenInGame` true :!label _label_3)
              (`self.SetActorEnableCollision` false)))
          (elif _returnvalue
            (goto _label_3)
            (else
              (goto _label_2))))))
    (:`CastFailed`
      (goto _label))))

(fn `UserConstructionScript`
  (bind _staticmesh (`self.StaticMesh`))
  (bind _isvisible (`self.IsVisible`))
  ;[1 1 1] Sets the platform the correct color, mesh, and visibility on construction
  (`PrimitiveComponent.SetMaterial` _staticmesh 0 (select `/Game/OldFiles/Character/Blueprints/ColorEnum` (`self.Color`) :`NewEnumerator5` "/Game/OldFiles/StarterContent/Materials/M_Basic_Floor.M_Basic_Floor" :`NewEnumerator0` "/Game/OldFiles/ColorChangeMechanics/Platforms/Materials/Red.Red" :`NewEnumerator1` "/Game/OldFiles/ColorChangeMechanics/Platforms/Materials/Blue.Blue" :`NewEnumerator2` "/Game/OldFiles/ColorChangeMechanics/Platforms/Materials/Yellow.Yellow" :!type "MaterialInterface Object Reference"))
  (`StaticMeshComponent.SetStaticMesh` _staticmesh (`self.Mesh`))
  (`SceneComponent.SetVisibility` _staticmesh _isvisible true)
  (`SceneComponent.SetVisibility` (`self.Selector`) (not _isvisible) true))