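; Grapple hook projectile with a cable to the player that latches the ColorSwapCharacter onto actors tagged "Grapple".
; Each tick, line traces from the player sweep the path since the last frame to catch missed hits.
; The GravitationField overlap steers velocity toward nearby tagged actors, ignoring those near the spawn point.
; GrappleConect passes tagged hits to a living character and destroys the hook on any actor hit.
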(event `self.ReceiveTick`
  (params (DeltaSeconds :type "Float (single-precision)"))
  (bind _returnvalue (`GameplayStatics.GetPlayerCharacter` 0))
  (bind _last_location (`self.Last Location`))
  (bind _projectile (`self.Projectile`))
  ;[1 1 1] Conect the grapple to gapplable objects
  (`|ExecutionSequence`
    (:`then_0`
      (for _index (range 21)
        (bind (_outhit _returnvalue_2) (`KismetSystemLibrary.LineTraceSingle` (`self.K2_GetActorLocation` _returnvalue) (`KismetMathLibrary.VLerp` _last_location (`self.K2_GetActorLocation`) (select `bool` (`KismetMathLibrary.EqualExactly_VectorVector` _last_location) :`false` (* _index 0.05) :`true` 1.0 :!type "Float (double-precision)")) "TraceTypeQuery1" false (`|MakeArray` _returnvalue :!type "Actor Object Reference") "None" true (struct :`R` 1.0 :`A` 1.0) (struct :`G` 1.0 :`A` 1.0) 20.0))
        (if _returnvalue_2
          (`self.GrappleConect` _outhit))))
    (:`then_1`
      (set `self.Last Location` (`self.K2_GetActorLocation`))
      ;[1 1 1] Homing
      (`/Engine/EditorBlueprintResources/StandardMacros.Gate` true :!label _label
        (:`Exit`
          (set `MovementComponent.Velocity` (+ (* (`KismetMathLibrary.GetDirectionUnitVector` (`self.K2_GetActorLocation`) (`.ImpactPoint` (`GameplayStatics.BreakHitResult` (`self.Hit`)))) 15.0) (`MovementComponent.Velocity` _projectile)) _projectile))))))

(event `self.ReceiveDestroyed`
  ;[1 1 1] Set Grapple in air to be false after destroyed
  (bind _ascolor_swap_character (cast `/Game/OldFiles/Character/Blueprints/ColorSwapCharacter` (`GameplayStatics.GetPlayerCharacter` 0)))
  (set `/Game/OldFiles/Character/Blueprints/ColorSwapCharacter.IsGrappleInAir` false _ascolor_swap_character))

(event `self.ReceiveHit`
  (params (MyComp :type "PrimitiveComponent Object Reference") (Other :type "Actor Object Reference") (OtherComp :type "PrimitiveComponent Object Reference") (bSelfMoved :type Boolean) (HitLocation :type "Vector Structure") (HitNormal :type "Vector Structure") (NormalImpulse :type "Vector Structure") (Hit :type "HitResult Structure (by ref)"))
  ;[1 1 1] Conect the grapple to gapplable objects
  (`self.GrappleConect` Hit))

(event `self.ReceiveBeginPlay`
  (bind _returnvalue (`self.K2_GetActorLocation`))
  ;[1 1 1] Attach Cable to player
  (`CableComponent.SetAttachEndTo` (`self.Cable`) (`GameplayStatics.GetPlayerCharacter` 0) "None" "None")
  ;[1 1 1] Make It so the grapple dosent home to somthing that you are next to
  (bind _outhits (`KismetSystemLibrary.SphereTraceMulti` _returnvalue _returnvalue 300.0 "TraceTypeQuery1"))
  (for _array_element _outhits
    (`KismetArrayLibrary.Array_Add` (`self.Inital Hit Actors`) (`.HitActor` (`GameplayStatics.BreakHitResult` _array_element)))))

(event `self.Gravitation Field.OnComponentBeginOverlap`
  (params (OverlappedComponent :type "PrimitiveComponent Object Reference") (OtherActor :type "Actor Object Reference") (OtherComp :type "PrimitiveComponent Object Reference") (OtherBodyIndex :type Integer) (bFromSweep :type Boolean) (SweepResult :type "HitResult Structure (by ref)"))
  (bind _returnvalue (`self.K2_GetActorLocation`))
  ;[1 1 1] Homing
  ;;[0.2026 1 0.2461] Start Homing
  (if (and (`self.ActorHasTag` OtherActor "Grapple") (not (`KismetArrayLibrary.Array_Contains` (`self.Inital Hit Actors`) OtherActor)))
    (`/Engine/EditorBlueprintResources/StandardMacros.DoOnce` false :!label _label_2
      (:`Completed`
        (bind _outhit (`KismetSystemLibrary.SphereTraceSingle` _returnvalue _returnvalue 300.0 "TraceTypeQuery1"))
        (set `self.Homing Actor` OtherActor)
        (set `self.Hit` _outhit)
        (goto _label :!via `Open`)))))

(event `self.Gravitation Field.OnComponentEndOverlap`
  (params (OverlappedComponent :type "PrimitiveComponent Object Reference") (OtherActor :type "Actor Object Reference") (OtherComp :type "PrimitiveComponent Object Reference") (OtherBodyIndex :type Integer))
  ;[1 1 1] Homing
  ;;[1 0.08333 0.08333] Stop Homing
  (if (and (`self.ActorHasTag` OtherActor "Grapple") (== OtherActor (`self.Homing Actor`)))
    (`|ExecutionSequence`
      (:`then_0`
        (goto _label_2 :!via `Reset`))
      (:`then_1`
        (goto _label :!via `Close`)))))

(fn `GrappleConect`
  (params (Hit :type "HitResult Structure"))
  (bind (_bblockinghit _binitialoverlap _time _distance _location _impactpoint _normal _impactnormal _physmat _hitactor) (`GameplayStatics.BreakHitResult` Hit))
  (bind _ascolor_swap_character (cast `/Game/OldFiles/Character/Blueprints/ColorSwapCharacter` (`GameplayStatics.GetPlayerCharacter` 0)))
  (if (not (`/Game/OldFiles/Character/Blueprints/ColorSwapCharacter.Dead` _ascolor_swap_character))
    (`/Engine/EditorBlueprintResources/StandardMacros.IsValid` _hitactor
      (:`Is Valid`
        (if (`self.ActorHasTag` _hitactor "Grapple")
          (set `/Game/OldFiles/Character/Blueprints/ColorSwapCharacter.IsGrapped` true _ascolor_swap_character)
          (set `/Game/OldFiles/Character/Blueprints/ColorSwapCharacter.GrappleHit` Hit _ascolor_swap_character)
          (set `/Game/OldFiles/Character/Blueprints/ColorSwapCharacter.GrappledActor` null _ascolor_swap_character))
        (`self.K2_DestroyActor`)))))

(fn `UserConstructionScript`)